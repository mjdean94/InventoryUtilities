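; Conan character component that pulls crafting or building ingredients from nearby containers into a target inventory.
; A sphere trace around the owner collects placeable containers the character owns and can access, skipping crafting stations with queued items.
; Ingredients come from visible crafting-panel widgets or the selected construction recipe, the latter filling the backpack.
; Each ingredient, scaled by quantity, is moved container by container until satisfied or sources run out.
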(event Custom|PullIngredients
  (params (TargetInventory :type Item%20Inventory%20Object%20Reference) (Ingredients :type Array%20of%20IU%20Ingredient%20Structures) (Quantity :type Integer))
  (CallFunction|PullIngredientListIntoInventory TargetInventory Ingredients Quantity))

(fn PullItemIntoInventory
  (params (SourceInventories :type Array%20of%20Item%20Inventory%20Object%20References) (TargetInventory :type Item%20Inventory%20Object%20Reference) (ItemTemplateId :type Integer) (Quantity :type Integer))
  (LocalVariables|SetQuantityRemaining Quantity)
  (for _array_element SourceInventories
    (bind _returnvalue (Class|ItemInventory|MoveItemsbyTemplateId _array_element ItemTemplateId (LocalVariables|GetQuantityRemaining) true TargetInventory false))
    (bind _output_get (LocalVariables|SetQuantityRemaining (- (LocalVariables|GetQuantityRemaining) _returnvalue)))
    (if (<= _output_get 0)
      (return))))

(fn PullIngredientListIntoInventory
  (params (TargetInventory :type Item%20Inventory%20Object%20Reference) (Ingredients :type Array%20of%20IU%20Ingredient%20Structures) (Quantity :type Integer))
  (bind _accessibleinventories (CallFunction|FindNearbyAccessibleInventories))
  (for _array_element Ingredients
    (CallFunction|PullItemIntoInventory _accessibleinventories TargetInventory (.itemid _array_element) (* (.quantity _array_element) Quantity))))

(fn FindNearbyAccessibleInventories
  (bind _returnvalue (Components|GetOwner))
  (bind _returnvalue_2 (Transformation|GetActorLocation _returnvalue))
  (bind _outhits (Collision|MultiSphereTraceByChannel _returnvalue_2 _returnvalue_2 1e+04 "TraceTypeQuery1" false 0 "ForDuration"))
  (for _array_element _outhits
    (bind _asbp_placeable_item_container (Utilities|Casting|CastToBP_PlaceableItemContainer (.hitactor _array_element)))
    (bind _isvalid (Validation|IsValidInventory _asbp_placeable_item_container))
    (if _isvalid
      (Utilities|Array|AddUnique (LocalVariables|GetResults) (Class|ItemInventory|GetInventorybyType (Variables|/Game/Systems/Building/Placeables/BP_PlaceableItemContainer.BP_PlaceableItemContainer_C|GetPlaceableInventory _asbp_placeable_item_container) _asbp_placeable_item_container (Variables|/Script/ConanSandbox.ItemInventory|GetInventoryType (Variables|/Game/Systems/Building/Placeables/BP_PlaceableItemContainer.BP_PlaceableItemContainer_C|GetPlaceableInventory _asbp_placeable_item_container))))))
  (return (LocalVariables|GetResults)))

(fn IsValidInventory
  (params (Candidate :type BP%20Placeable%20Item%20Container%20Object%20Reference))
  (bind _asconan_character (Utilities|Casting|CastToConanCharacter (Components|GetOwner)))
  (bind _isactive (Validation|IsActiveCraftingStation Candidate))
  (return (Math|Boolean|ANDBoolean (not _isactive) (.CanAccess (Class|PlaceableBase|CanAccessContainer Candidate _asconan_character)) (Class|BuildableBase|IsOwner Candidate _asconan_character false))))

(fn IsActiveCraftingStation
  (params (Candidate :type BP%20Placeable%20Item%20Container%20Object%20Reference))
  (bind _asbp_pl_crafting_station (Utilities|Casting|CastToBP_PL_Crafting_Station Candidate)
    (:then
      (return (> (Utilities|Array|Length (Variables|/Script/ConanSandbox.ItemInventory|GetItemList (Variables|/Game/Systems/Building/Placeables/BP_PL_Crafting_Station.BP_PL_Crafting_Station_C|GetCraftingQueue _asbp_pl_crafting_station))) 0)))
    (:CastFailed
      (return false))))

(fn HandleCooldown
  (params (DeltaTime :type Float%20%28single-precision%29))
  (if (> (Variables|Default|GetPullCooldown) 0.0)
    (Variables|Default|SetPullCooldown (- (Variables|Default|GetPullCooldown) DeltaTime))))

(fn GetCraftingPanelRecipeIngredients
  (bind _foundwidgets (Widget|GetAllWidgetsOfClass "/Game/UI/Inventory/W_CraftingIngredientIconView.W_CraftingIngredientIconView_C" false))
  (for _array_element _foundwidgets
    (if (Widget|IsVisible _array_element)
      (Utilities|Array|Add (LocalVariables|GetResults) (Utilities|Struct|MakeIU_Ingredient (Variables|/Script/ConanSandbox.GameItem|GetTemplateID (Class|InventoryIconViewBase|GetItem _array_element)) (Class|GameItem|GetIntStat (Class|InventoryIconViewBase|GetItem _array_element) "StackSize")))))
  (return (LocalVariables|GetResults)))

(fn BuildRecipeIngredientList
  (params (Recipe :type Recipe%20Item%20Object%20Reference))
  (for _array_element (Variables|/Script/ConanSandbox.RecipeItem|GetIngredients Recipe)
    (Utilities|Array|Add (LocalVariables|GetResults) (Utilities|Struct|MakeIU_Ingredient (.ingredientid _array_element) (.ingredientquantity _array_element))))
  (return (LocalVariables|GetResults)))

(fn PullCraftingPanelIngredients
  (params (TargetInventory :type Item%20Inventory%20Object%20Reference) (Quantity :type Integer))
  (bind _ingredientlist (CallFunction|GetCraftingPanelRecipeIngredients))
  (CallFunction|PullIngredients TargetInventory _ingredientlist Quantity))

(fn GetNeededQuantity
  (params (TargetInventory :type Item%20Inventory%20Object%20Reference) (ItemTemplateId :type Integer) (Stacksize :type Integer) (Quantity :type Integer))
  (return (Math|Integer|Max(Integer) (- (* Stacksize Quantity) (Class|ItemInventory|GetNumberOfItemsbyTemplate TargetInventory ItemTemplateId)))))

(fn PullConstructionIngredients
  (params (Quantity :type Integer))
  (bind _asconan_character (Utilities|Casting|CastToConanCharacter (Components|GetOwner)))
  (bind _returnvalue (Class|ConanCharacter|GetBuildSystemComponent _asconan_character))
  (if (Utilities|Enum|Equal(Enum) (Variables|/Script/ConanSandbox.BuildSystemComponent|GetConstructionMode _returnvalue) "Construction")
    (Utilities|IsValid (Variables|/Script/ConanSandbox.BuildSystemComponent|GetConstructionModeSelectedRecipe _returnvalue)
      (:Is%20Valid
        (bind _ingredientlist (Helper|BuildRecipeIngredientList (Variables|/Script/ConanSandbox.BuildSystemComponent|GetConstructionModeSelectedRecipe _returnvalue)))
        (bind _returnvalue_2 (Class|ConanCharacter|GetBackpackInventory _asconan_character))
        (CallFunction|PullIngredients _returnvalue_2 _ingredientlist Quantity)))))