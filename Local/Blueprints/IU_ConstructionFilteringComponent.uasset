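; Character component that adds name search filtering to the construction GUI's recipe list.
; On GUI open it caches the character's full recipe inventory, then applies the current search text, which is also restored to the searchbox on initialization.
; Filtering overwrites the displayed inventory's ItemList with name matches (all items if empty) and refreshes the view.
; Closing the GUI writes the cached full list back to the recipe inventory.
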(event Custom|OnGuiClosed
  (params (window :type Window%20Root%20Object%20Reference))
  (bind _returnvalue (Class|ConanCharacter|GetRecipeInventory (Variables|Default|GetCharacterReference) false))
  (Variables|/Script/ConanSandbox.ItemInventory|SetItemList _returnvalue (Variables|Default|GetFullInventory)))

(event Custom|OnGuiOpened
  (params (window :type Window%20Root%20Object%20Reference))
  (bind _returnvalue (Class|ConanCharacter|GetRecipeInventory (Variables|Default|GetCharacterReference) false))
  (Variables|Default|SetFullInventory (Variables|/Script/ConanSandbox.ItemInventory|GetItemList _returnvalue))
  (CallFunction|ApplyFilter))

(event Custom|OnConstructionGuiInitialized
  (bind _constructiongui (Variables|Default|GetConstructionGui))
  (Class|FCEditableTextBox|SetText (Variables|/Game/Mods/InventoryUtilities/UI/IU_ConstructionGui.IU_ConstructionGui_C|GetSearchbox (Variables|Default|GetConstructionGui)) (Variables|Default|GetCurrentFilterText))
  (EventDispatchers|BindEventtoSignalClosing _constructiongui (delegate Custom|OnGuiClosed))
  (EventDispatchers|BindEventtoSignalOpened _constructiongui (delegate Custom|OnGuiOpened)))

(event EventBeginPlay
  (bind _asconan_character (Utilities|Casting|CastToConanCharacter (Components|GetOwner)))
  (Utilities|IsValid _asconan_character
    (:Is%20Valid
      (Variables|Default|SetCharacterReference _asconan_character))
    (:Is%20Not%20Valid
      (Components|DestroyComponent))))

(fn SetFilter
  (params (NewFilterText :type Text))
  (Variables|Default|SetCurrentFilterText NewFilterText)
  (CallFunction|ApplyFilter))

(fn InitializeConstructionGui
  (params (NewConstructionGui :type IU%20Construction%20Gui%20Object%20Reference))
  (Variables|Default|SetConstructionGui NewConstructionGui)
  (CallFunction|OnConstructionGuiInitialized))

(fn ApplyFilter
  (bind _constructiongui (Variables|Default|GetConstructionGui))
  (bind _constructioninventoryview (Variables|/Script/ConanSandbox.ConstructionGuiBase|GetConstructionInventoryView _constructiongui))
  (bind _inventory (Variables|/Script/ConanSandbox.InventoryGridViewBase|GetInventory _constructioninventoryview))
  (Utilities|IsValid (Variables|/Script/ConanSandbox.InventoryGridViewBase|GetInventory (Variables|/Script/ConanSandbox.ConstructionGuiBase|GetConstructionInventoryView (Variables|Default|GetConstructionGui)))
    (:Is%20Valid
      (for _array_element (Variables|Default|GetFullInventory)
        (Utilities|Or+Branch (Utilities|Enum|Equal(Enum) (Utilities|String|ToString(Text) (Variables|Default|GetCurrentFilterText)) "") (Utilities|String|Contains (Utilities|String|ToString(Text) (Class|GameItem|GetItemName _array_element)) (Utilities|String|ToString(Text) (Variables|Default|GetCurrentFilterText)))
          (:True
            (Utilities|Array|Add (LocalVariables|GetResult) _array_element))))
      (Variables|/Script/ConanSandbox.ItemInventory|SetItemList _inventory (LocalVariables|GetResult))
      (Class|InventoryGridViewBase|SetInventory _constructioninventoryview _inventory)
      (Default|RefreshSubclasses _constructiongui))))