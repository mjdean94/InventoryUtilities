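; IU_Input handles player input for pulling construction ingredients through the IU_InventoryUtilitiesComponent on its owner.
; Releasing InteractKey calls that component's PullConstructionIngredients with the current amount, which Sprint switches between a larger batch while held and a single item on release.
; Tick counts down a PullCooldown, though nothing in this graph sets or checks it.
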(event EventTick
  (params (DeltaSeconds :type Float%20%28single-precision%29))
  (if (> (Variables|Default|GetPullCooldown) 0.0)
    (Variables|Default|SetPullCooldown (- (Variables|Default|GetPullCooldown) DeltaSeconds))))

(event Input|ActionEvents|InputActionInteractKey
  (params (Key :type Key%20Structure :default "AnyKey"))
  (:Released
    (Default|PullConstructionIngredients (Actor|GetComponentbyClass (Components|GetOwner) "/Game/Mods/InventoryUtilities/Blueprints/IU_InventoryUtilitiesComponent.IU_InventoryUtilitiesComponent_C") (Variables|Default|GetAmountToPull))))

(event Input|ActionEvents|InputActionSprint
  (params (Key :type Key%20Structure :default "AnyKey"))
  (:Pressed
    (Variables|Default|SetAmountToPull 5))
  (:Released
    (Variables|Default|SetAmountToPull 1)))