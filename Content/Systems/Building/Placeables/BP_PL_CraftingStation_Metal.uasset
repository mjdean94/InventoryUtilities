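; Metal crafting station placeable that supports artisan thralls and randomizes the stats of flagged items added to its inventory.
; The blacksmith work slot state hides props while in use and, together with the crafting queue, switches the station lights.
; A StaminaClimbingCostMultiplier of 10 acts as a one-time flag: such items get weapon stamina, damage, durability, armor penetration and weight scaled randomly per group, then the flag resets.
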(event SignalItemAdded(PlaceableInventory)
  (params (index :type Integer) (item :type Game%20Item%20Object%20Reference) (srcInventory :type Item%20Inventory%20Object%20Reference) (srcIndex :type Integer))
  (Variables|Default|SetItemToModify item)
  (if (== (Class|GameItem|GetFloatStat item "StaminaClimbingCostMultiplier") 1e+01)
    (CallFunction|ModifyIntStat (Variables|Default|GetItemToModify) 0.85 1.15 (Utilities|Array|MakeArray "WeaponStaminaAttackSingleBasic" "WeaponStaminaAttackSingleSpecial" "WeaponStaminaAttackDualBasic" "WeaponStaminaAttackDualSpecial"))
    (CallFunction|ModifyIntStat (Variables|Default|GetItemToModify) 0.85 1.15 (Utilities|Array|MakeArray "DamageHealthLight_OnHit" "DamageHealthHeavy_OnHit"))
    (CallFunction|ModifyFloatStat (Variables|Default|GetItemToModify) 0.85 1.15 (Utilities|Array|MakeArray "MaxDurability"))
    (Class|GameItem|SetFloatStat (Variables|Default|GetItemToModify) "CurrentDurability" (Class|GameItem|GetFloatStat (Variables|Default|GetItemToModify) "MaxDurability") true)
    (CallFunction|ModifyFloatStat (Variables|Default|GetItemToModify) 0.85 1.15 (Utilities|Array|MakeArray "ArmorPen"))
    (CallFunction|ModifyFloatStat (Variables|Default|GetItemToModify) 0.85 1.15 (Utilities|Array|MakeArray "EncumbranceWeight"))
    (Class|GameItem|SetFloatStat (Variables|Default|GetItemToModify) "StaminaClimbingCostMultiplier" 1.0 true)))

(event Custom|SlotStateChanged
  (params (SlotComponent :type Smart%20Object%20Slot%20Component%20Object%20Reference) (PrevState :type ESmartObjectSlotState%20Enum) (NewState :type ESmartObjectSlotState%20Enum))
  (bind _bp_bac_turnlightonoff (Variables|Default|GetBP_BAC_TurnLightOnOff))
  (switch Utilities|FlowControl|Switch|SwitchonESmartObjectSlotState NewState
    (:Deactivated
      (CallFunction|TogglePropVisibility true :!label _label)
      (if (Class|CraftingQueue|IsRunning (Variables|Default|GetCraftingQueue))
        (Default|TurnonAll _bp_bac_turnlightonoff)
        (else
          (Default|TurnOffAll _bp_bac_turnlightonoff))))
    (:Available
      (goto _label))
    (:Reserved
      (goto _label))
    (:InUse
      (CallFunction|TogglePropVisibility false)
      (Default|TurnonAll (Variables|Default|GetBP_BAC_TurnLightOnOff)))))

(event EventBeginPlay
  (if (not (Class|CraftingQueue|IsRunning (Variables|Default|GetCraftingQueue)))
    (Default|TurnOffAll (Variables|Default|GetBP_BAC_TurnLightOnOff)))
  (|CallParentFunction)
  (if (not (Variables|Default|GetIsABrush))
    (EventDispatchers|BindEventtoOnStateChanged (Variables|Default|GetSOS_Work_Blacksmith) (delegate Custom|SlotStateChanged))
    (CallFunction|SlotStateChanged 0 "Deactivated" (Class|SmartObjectSlotComponent|GetState (Variables|Default|GetSOS_Work_Blacksmith)))))

(event EventEndPlay
  (params (EndPlayReason :type EEndPlayReason%20Enum :default "Destroyed"))
  (|CallParentFunction EndPlayReason)
  (EventDispatchers|UnbindallEventsfromOnStateChanged (Variables|Default|GetSOS_Work_Blacksmith)))

(fn ConstructionScript
  (|CallParentFunction))

(fn GetArtisanThrallInventory
  (return (Variables|Default|GetThrallInventory)))

(fn ModifyFloatStat
  (params (Target :type Game%20Item%20Object%20Reference) (Min :type Float%20%28single-precision%29) (Max :type Float%20%28single-precision%29) (InputPin :type Array%20of%20EItemFloatStatID%20Enums))
  (LocalVariables|SetLocal_Multiplier (Math|Random|RandomFloatinRange Min Max))
  (for _array_element InputPin
    (Class|GameItem|SetFloatStat Target _array_element (* (Class|GameItem|GetFloatStat Target _array_element) (LocalVariables|GetLocal_Multiplier)) true)))

(fn ModifyIntStat
  (params (Target :type Game%20Item%20Object%20Reference) (Min :type Float%20%28single-precision%29) (Max :type Float%20%28single-precision%29) (InputPin :type Array%20of%20EItemIntStatID%20Enums))
  (LocalVariables|SetLocal_Multiplier (Math|Random|RandomFloatinRange Min Max))
  (for _array_element InputPin
    (Class|GameItem|SetIntStat Target _array_element (Math|Float|Truncate (* (Class|GameItem|GetIntStat Target _array_element) (LocalVariables|GetLocal_Multiplier))) true)))

(fn CanStationUseThralls
  (return true))